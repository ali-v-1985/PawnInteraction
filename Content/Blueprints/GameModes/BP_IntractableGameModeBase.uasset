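; BP_IntractableGameModeBase is a game mode Blueprint that scatters spawned actors across the level when play begins.
; BeginPlay calls SpawnActors, which loops over NumberOfActors and spawns at random X and Y positions at a fixed height.
; The random range is MapSize multiplied by the loop index, so the first actor lands at the X/Y origin and later ones can land progressively farther out.
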(event EventBeginPlay
  (CallFunction|SpawnActors))

(event EventTick
  (params (DeltaSeconds :type Float%20%28single-precision%29)))

(fn ConstructionScript)

(fn SpawnActors
  (bind _map_size (Variables|Default|GetMap%20Size))
  (for _index (range 0 (Variables|Default|GetNumberOfActors))
    (Game|SpawnActorfromClass 0 (Math|Transform|MakeTransform (Math|Vector|MakeVector (Math|Random|RandomFloatinRange (* _index (* -1 _map_size)) (* _index _map_size)) (Math|Random|RandomFloatinRange (* _index (* -1 _map_size)) (* _index _map_size)) 2e+01) "0, 0, 0" "1,1,1") "Undefined" 0 0)))